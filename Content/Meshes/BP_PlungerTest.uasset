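; BP_PlungerTest is a test plunger actor that pulls a cube back while Enter is held and returns it on release.
; The Pullback timeline lerps the cube from its construction-time location along world X by PlungerStart.
; Releasing Enter reverses the timeline from its current position at PLungerSpeed.
; The cube is moved by setting its world location directly, without sweep or physics teleport.
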(event EventBeginPlay)

(event Collision|EventActorBeginOverlap
  (params (OtherActor :type Actor%20Object%20Reference)))

(event EventTick
  (params (DeltaSeconds :type Float%20%28single-precision%29)))

(event Input|KeyboardEvents|Enter
  (params (Key :type Key%20Structure))
  (bind _startloc (Variables|Default|GetStartLoc))
  (bind _pullback (Variables|Default|GetPullback))
  (:Pressed
    (Components|Timeline|SetPlayRate _pullback 1.0)
    (bind _newtrack_1 (Timeline|Pullback PlayFromStart)
      (:Update
        (Transformation|SetWorldLocation (Variables|Default|GetCube) (Math|Vector|Lerp(Vector) _startloc (+ _startloc (Math|Vector|MakeVector (Variables|Default|GetPlungerStart) 0.0 0.0)) _newtrack_1) false false))))
  (:Released
    (Components|Timeline|SetPlayRate _pullback (Variables|Default|GetPLungerSpeed))
    (Timeline|Pullback Reverse)))

(fn ConstructionScript
  (Variables|Default|SetStartLoc (Transformation|GetWorldLocation (Variables|Default|GetCube))))