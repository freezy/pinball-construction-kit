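; BP_KickerHole is a pinball kicker hole that traps a ball, holds it, then kicks it back out for points.
; Capsule overlap marks the ball trapped, stops its physics and uses a timeline to lerp it to the hole's center.
; After TrapTime, PopBall restores physics, launches the ball along KickDirection with upward velocity and registers score.
; Capsule overlaps switch off during the hold and re-enable shortly after the kick.
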(event OnComponentBeginOverlap(Capsule)
  (params (OverlappedComponent :type Primitive%20Component%20Object%20Reference) (OtherActor :type Actor%20Object%20Reference) (OtherComp :type Primitive%20Component%20Object%20Reference) (OtherBodyIndex :type Integer) (bFromSweep :type Boolean) (SweepResult :type Hit%20Result%20Structure%20%28by%20ref%29))
  (bind _returnvalue (Transformation|GetActorLocation))
  (bind (_x _y _z) (Math|Vector|BreakVector _returnvalue))
  (bind _asbase_pinball (Utilities|Casting|CastToBasePinball OtherActor))
  (bind _output_get (Variables|Default|SetTrappedBall _asbase_pinball))
  (Variables|/Game/Blueprints/BasePinball.BasePinball_C|SetBallTrapped _asbase_pinball true)
  (Physics|SetSimulatePhysics (Variables|/Script/Pinball.PinballBall|GetBall _asbase_pinball) false)
  (Class|PrimitiveComponent|SetAllPhysicsLinearVelocity (Variables|/Script/Pinball.PinballBall|GetBall _asbase_pinball) "0, 0,0.000000" false)
  (Class|PrimitiveComponent|SetPhysicsAngularVelocityinDegrees (Variables|/Script/Pinball.PinballBall|GetBall _asbase_pinball) "0, 0, 0" false "None")
  (Variables|Default|SetStartLoc (Transformation|GetActorLocation _output_get))
  (bind _newtrack_0 (Timeline|QuickPositionLerp PlayFromStart)
    (:Update
      (Transformation|SetActorLocation _asbase_pinball (Math|Vector|Lerp(Vector) (Variables|Default|GetStartLoc) (Math|Vector|MakeVector _x _y (- _z 0.0)) _newtrack_0) false false))
    (:Finished
      (Audio|PlaySoundatLocation "/Game/Assets/Audio/FireWeapon_ImpactHiss04.FireWeapon_ImpactHiss04" _returnvalue)
      (Variables|/Script/Engine.PrimitiveComponent|SetbGenerateOverlapEvents (Variables|Default|GetCapsule) false)
      (Utilities|Time|SetTimerbyFunctionName 0 "PopBall" (Variables|Default|GetTrapTime)))))

(event Custom|PopBall
  (bind _trappedball (Variables|Default|GetTrappedBall))
  (bind _kickdirection (Variables|Default|GetKickDirection))
  (bind _returnvalue (* _kickdirection 2.0))
  (bind _ball (Variables|/Script/Pinball.PinballBall|GetBall _trappedball))
  (Collision|SetCollisionEnabled _ball "QueryAndPhysics")
  (Physics|SetSimulatePhysics _ball true)
  (Physics|SetPhysicsLinearVelocity _ball (Math|Vector|MakeVector (.x _returnvalue) (.y _returnvalue) 2.5e+02) false "None")
  (Variables|/Game/Blueprints/BasePinball.BasePinball_C|SetBallTrapped _trappedball false)
  (Audio|PlaySoundatLocation "/Game/Assets/Audio/Door_Lock03.Door_Lock03" (Transformation|GetActorLocation))
  (Default|RegisterScore (Variables|Default|GetScoreComponent))
  (Utilities|FlowControl|Delay 1.0)
  (Variables|/Script/Engine.PrimitiveComponent|SetbGenerateOverlapEvents (Variables|Default|GetCapsule) true))

(event EventBeginPlay)

(event Collision|EventActorBeginOverlap
  (params (OtherActor :type Actor%20Object%20Reference)))

(event EventTick
  (params (DeltaSeconds :type Float%20%28single-precision%29)))

(fn ConstructionScript)