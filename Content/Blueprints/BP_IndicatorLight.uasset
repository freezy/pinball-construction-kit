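; BP_IndicatorLight is an indicator light actor with a point light and a mesh showing a configurable icon and letter, starting unlit at BeginPlay.
; The construction script sets light color and builds a dynamic material instance for the textures, with a TestLit preview option.
; Activate and Deactivate store the logical state, switch light visibility and emissive power, and notify an optional light group.
; ResetLightState restores the visuals from that state after light effects.
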(event Custom|ResetLightState
  (if (Variables|Default|GetLightActive)
    (CallFunction|Turnon)
    (else
      (CallFunction|TurnOff))))

(event EventActivate
  (bind _mylightgroup (Variables|Default|GetMyLightGroup))
  (Variables|Default|SetLightActive true)
  (CallFunction|Turnon)
  (Utilities|IsValid _mylightgroup
    (:Is%20Valid
      (Default|NotifyLitUnlit _mylightgroup true))))

(event EventBeginPlay
  (CallFunction|Deactivate))

(event EventActorBeginOverlap
  (params (OtherActor :type Actor%20Object%20Reference)))

(event EventTick
  (params (DeltaSeconds :type Float%20%28single-precision%29)))

(event EventDeactivate
  (bind _mylightgroup (Variables|Default|GetMyLightGroup))
  (Variables|Default|SetLightActive false)
  (CallFunction|TurnOff)
  (Utilities|IsValid _mylightgroup
    (:Is%20Valid
      (Default|NotifyLitUnlit _mylightgroup false))))

(fn ConstructionScript
  (bind _indicatormesh (Variables|Default|GetIndicatorMesh))
  (Rendering|Components|Light|SetLightColor (Variables|Default|GetPointLight) (Variables|IndicatorLight|GetLightColor) true)
  (Rendering|Material|SetMaterial _indicatormesh 0 (Variables|IndicatorLight|GetIndicatorMaterial))
  (bind _returnvalue (Rendering|Material|CreateDynamicMaterialInstance _indicatormesh 0 0 :!class /Script/Engine.PrimitiveComponent))
  (bind _output_get (Variables|Default|SetIndicatorMID _returnvalue))
  (Rendering|Material|SetScalarParameterValue _output_get "LightPower" 0.0 :!class /Script/Engine.MaterialInstanceDynamic)
  (Rendering|Material|SetTextureParameterValue _output_get "IconTexture" (Variables|IndicatorLight|GetIconTexture))
  (Rendering|Material|SetTextureParameterValue _output_get "LetterTexture" (Utilities|Array|Get(acopy) (Variables|Default|GetLetterTextures) (Math|Conversions|ToInteger(Byte) (Variables|IndicatorLight|GetUseLetter))))
  (if (Variables|IndicatorLight|GetTestLit)
    (CallFunction|Activate)))

(fn Turnon
  (Rendering|SetVisibility (Variables|Default|GetPointLight) true false)
  (Rendering|Material|SetScalarParameterValue (Variables|Default|GetIndicatorMID) "LightPower" 5.0 :!class /Script/Engine.MaterialInstanceDynamic))

(fn TurnOff
  (Rendering|SetVisibility (Variables|Default|GetPointLight) false false)
  (Rendering|Material|SetScalarParameterValue (Variables|Default|GetIndicatorMID) "LightPower" 0.0 :!class /Script/Engine.MaterialInstanceDynamic))