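; BP_MiscTrigger is a pinball trigger that fires when a BasePinball overlaps it.
; The overlap plays a sound, lights the indicator, sends ActivateMessage to ObjectToActivate, registers score and starts a special mode through components.
; The construction script creates the indicator's dynamic material with its icon and the light off.
; A FlipFlop toggle for deactivation is left unwired, so overlaps only activate.
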(event OnComponentBeginOverlap(Trigger)
  (params (OtherActor :type Actor%20Object%20Reference) (OtherComp :type Primitive%20Component%20Object%20Reference) (OtherBodyIndex :type Integer) (bFromSweep :type Boolean) (SweepResult :type Hit%20Result%20Structure%20%28by%20ref%29))
  (Utilities|Casting|CastToBasePinball OtherActor)
  (Audio|PlaySoundatLocation (Variables|Default|GetActivationSound) (Transformation|GetActorLocation))
  (CallFunction|Activate)
  (Class|PinballInterface|Activate(Message) (Variables|Default|GetObjectToActivate))
  ;[1 1 1] Add Points and start any special mode
  (Default|RegisterScore (Variables|Default|GetScoreComponent))
  (Default|StartSpecialMode (Variables|Default|GetSpecialModeComponent) "NewEnumerator9" false))

(event EventActivate
  (Rendering|Material|SetScalarParameterValue (Variables|Default|GetIndicatorMID) "LightPower" 4.0 :!class /Script/Engine.MaterialInstanceDynamic))

(event EventBeginPlay)

(event Collision|EventActorBeginOverlap
  (params (OtherActor :type Actor%20Object%20Reference)))

(event EventTick
  (params (DeltaSeconds :type Float%20%28single-precision%29)))

(event EventDeactivate
  (Rendering|Material|SetScalarParameterValue (Variables|Default|GetIndicatorMID) "LightPower" 0.0 :!class /Script/Engine.MaterialInstanceDynamic))

(fn ConstructionScript
  (bind _indicatormesh (Variables|Default|GetIndicatorMesh))
  (Rendering|Material|SetMaterial _indicatormesh 0 (Variables|Default|GetIndicatorMaterial))
  (bind _returnvalue (Rendering|Material|CreateDynamicMaterialInstance _indicatormesh 0 0 :!class /Script/Engine.PrimitiveComponent))
  (bind _output_get (Variables|Default|SetIndicatorMID _returnvalue))
  (Rendering|Material|SetScalarParameterValue _output_get "LightPower" 0.0 :!class /Script/Engine.MaterialInstanceDynamic)
  (Rendering|Material|SetTextureParameterValue _output_get "IconTexture" (Variables|Default|GetIconTexture)))