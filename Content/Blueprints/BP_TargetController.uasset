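; BP_TargetController tracks downed targets across several target sets and triggers a special mode once all of them are down.
; On BeginPlay it registers itself with each set in TargetSets and totals their target counts.
; NotifyTargetDowned increments a counter; on reaching the total, it resets every set and the count, plays an arcade sound, and calls StartSpecialMode on SpecialModeComponent.
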(event Custom|ResetAlltargetSets
  ;[1 1 1] Reset All targets on Sets
  (for _array_element (Variables|Default|GetTargetSets)
    (Default|Resettargets _array_element)
    (Variables|Default|SetDownedTargets 0))
  (Audio|PlaySoundatLocation "/Game/Sounds/Arcade_GameStart.Arcade_GameStart" (Transformation|GetActorLocation)))

(event Custom|NotifyTargetDowned
  (bind _result (Math|Integer|IncrementInt (Variables|Default|GetDownedTargets))
    (:%20%20
      (if (== _result (Variables|Default|GetTotalTargets))
        (CallFunction|ResetAlltargetSets)
        (CallFunction|StartSpecial)))))

(event Custom|StartSpecial
  (Default|StartSpecialMode (Variables|Default|GetSpecialModeComponent) "NewEnumerator9" false))

(event EventBeginPlay
  (for _array_element (Variables|Default|GetTargetSets)
    (Variables|/Game/Blueprints/BP_TargetSet.BP_TargetSet_C|SetMyTargetController _array_element self)
    (Variables|Default|SetTotalTargets (+ (Variables|/Game/Blueprints/BP_TargetSet.BP_TargetSet_C|GetNumberOfTargets _array_element) (Variables|Default|GetTotalTargets)))))

(event EventActorBeginOverlap
  (params (OtherActor :type Actor%20Object%20Reference)))

(event EventTick
  (params (DeltaSeconds :type Float%20%28single-precision%29)))

(fn ConstructionScript)