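; Blueprint function library that builds walls and a flat top cap from a spline, apparently for pinball spline actors.
; AddSplineMeshComponents rebuilds one height-scaled spline mesh per segment, closing looped splines, with per-segment materials defaulting to numbered wall textures and aspect set from length over height.
; CreateProceduralMeshForPlanarVertices samples subdivided spline points, triangulates them via C++ ear clipping, reverses winding and builds a procedural cap with bounds-normalized UVs.
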(fn AddSplineMeshComponents
  (params (InSplineComponent :type Spline%20Component%20Object%20Reference) (InSplineActor :type Spline%20Actor%20Object%20Reference) (InHeight :type Float%20%28single-precision%29) (InSideMaterials :type Array%20of%20Material%20Interface%20Object%20References) (InNumberTextures :type Array%20of%20Texture%202D%20Object%20References) (InStaticMesh :type Static%20Mesh%20Object%20Reference) (ZeroMatAllWalls :type Boolean))
  (Utilities|FlowControl|Sequence
    (:then_0
      (LocalVariables|SetSpline%20Component InSplineComponent))
    (:then_1
      (bind _output_get (LocalVariables|SetSplineActor InSplineActor)))
    (:then_2
      (LocalVariables|SetHeight InHeight))
    (:then_3
      (LocalVariables|SetSideMaterials InSideMaterials))
    (:then_4
      (LocalVariables|SetNumberTextures InNumberTextures))
    (:then_5
      (LocalVariables|SetMeshToUse InStaticMesh))
    (:then_6
      (LocalVariables|SetUseMaterialZeroForAllWalls ZeroMatAllWalls))
    (:then_7
      (Class|SplineActor|DestroyAllSplineMeshes _output_get)
      ;[1 1 1] Loop through each spline segment
      (for _index (range 0 (- (Spline|GetNumberOfSplinePoints (LocalVariables|GetSpline%20Component)) 1))
        (LocalVariables|SetSpline%20Point%20Index _index)
        (bind _output_get_2 (LocalVariables|SetPrevious%20Spline%20Point%20Index (- _index 1)))
        (if (< _output_get_2 0)
          ;[1 1 1] Conditionally close the loop
          (LocalVariables|SetPrevious%20Spline%20Point%20Index (- (Spline|GetNumberOfSplinePoints (LocalVariables|GetSpline%20Component)) 1))
          (if (Class|SplineComponent|IsClosedLoop (LocalVariables|GetSpline%20Component))
            ;[1 1 1] Create Spline Mesh Component and set collision, static mesh, positions and tangents
            (bind _returnvalue (Class|SplineActor|AddPinballSplineMeshComponent (LocalVariables|GetSplineActor) false :!label _label))
            (Utilities|FlowControl|Sequence
              (:then_0
                (Collision|SetCollisionProfileName _returnvalue "BlockAll" :!class /Script/Engine.PrimitiveComponent))
              (:then_1
                (Components|StaticMesh|SetStaticMesh _returnvalue (LocalVariables|GetMeshToUse)))
              (:then_2
                (SplineMesh|SetStartandEnd _returnvalue (Spline|GetLocationatSplinePoint (LocalVariables|GetSpline%20Component) (LocalVariables|GetPrevious%20Spline%20Point%20Index) "Local") (Spline|GetTangentatSplinePoint (LocalVariables|GetSpline%20Component) (LocalVariables|GetPrevious%20Spline%20Point%20Index) "Local") (Spline|GetLocationatSplinePoint (LocalVariables|GetSpline%20Component) (LocalVariables|GetSpline%20Point%20Index) "Local") (Spline|GetTangentatSplinePoint (LocalVariables|GetSpline%20Component) (LocalVariables|GetSpline%20Point%20Index) "Local") :!class /Script/Engine.SplineMeshComponent)
                (LocalVariables|SetSplineLength (Math|Vector|VectorLength (- (Spline|GetLocationatSplinePoint (LocalVariables|GetSpline%20Component) (LocalVariables|GetSpline%20Point%20Index) "Local") (Spline|GetLocationatSplinePoint (LocalVariables|GetSpline%20Component) (LocalVariables|GetPrevious%20Spline%20Point%20Index) "Local")))))
              (:then_3
                ;[1 1 1] Save these vertices to use later to make a top
                (Utilities|Array|Add (LocalVariables|GetSplinePointVertices) (Math|Vector|MakeVector (.X (Math|Vector|BreakVector (Spline|GetLocationatSplinePoint (LocalVariables|GetSpline%20Component) (LocalVariables|GetPrevious%20Spline%20Point%20Index) "Local"))) (.Y (Math|Vector|BreakVector (Spline|GetLocationatSplinePoint (LocalVariables|GetSpline%20Component) (LocalVariables|GetPrevious%20Spline%20Point%20Index) "Local"))) 0.0))
                (Transformation|SetRelativeScale3D _returnvalue (Math|Vector|MakeVector 1.0 1.0 (/ (LocalVariables|GetHeight) 1e+02))))
              (:then_4
                ;[1 1 1] For each Spline Segment, if material exists, apply it. If it doesn't exist, add a numbered material
                (if (LocalVariables|GetUseMaterialZeroForAllWalls)
                  (Utilities|Array|SetArrayElem (LocalVariables|GetSideMaterials) (LocalVariables|GetSpline%20Point%20Index) (Utilities|Array|Get(acopy) (LocalVariables|GetSideMaterials)) true)
                  (else
                    (Utilities|IsValid (Utilities|Array|Get(acopy) (LocalVariables|GetSideMaterials) (LocalVariables|GetSpline%20Point%20Index))
                      (:Is%20Valid
                        _)
                      (:Is%20Not%20Valid
                        (bind _returnvalue_2 (Rendering|Material|CreateDynamicMaterialInstance 0 "/Game/Materials/M_WallMat.M_WallMat" :!class /Script/Engine.KismetMaterialLibrary))
                        (Rendering|Material|SetTextureParameterValue _returnvalue_2 "FirstDigit" (Utilities|Array|Get(acopy) (LocalVariables|GetNumberTextures) (.ReturnValue (Math|Float|Division(WholeandRemainder) (Math|Conversions|ToFloat(Integer) (LocalVariables|GetSpline%20Point%20Index)) 1e+01))))
                        (Rendering|Material|SetTextureParameterValue _returnvalue_2 "SecondDigit" (Utilities|Array|Get(acopy) (LocalVariables|GetNumberTextures) (Math|Float|Truncate (.Remainder (Math|Float|Division(WholeandRemainder) (Math|Conversions|ToFloat(Integer) (LocalVariables|GetSpline%20Point%20Index)) 1e+01)))))
                        (Utilities|Array|SetArrayElem (LocalVariables|GetSideMaterials) (LocalVariables|GetSpline%20Point%20Index) _returnvalue_2 true)))))
                (Rendering|Material|SetMaterial _returnvalue 0 (Utilities|Array|Get(acopy) (LocalVariables|GetSideMaterials) (LocalVariables|GetSpline%20Point%20Index)))
                ;[1 1 1] Try to normalize the texture aspect ratio based on spline length
                (bind _returnvalue_3 (Rendering|Material|CreateDynamicMaterialInstance _returnvalue 0 0 :!class /Script/Engine.PrimitiveComponent))
                (Rendering|Material|SetScalarParameterValue _returnvalue_3 "Aspect" (/ (LocalVariables|GetSplineLength) (LocalVariables|GetHeight)) :!class /Script/Engine.MaterialInstanceDynamic))))
          (else
            (goto _label))))
      (return (LocalVariables|GetSplinePointVertices) (LocalVariables|GetSideMaterials)))))

(fn CreateProceduralMeshforPlanarVertices
  (params (In%20Height :type Float%20%28single-precision%29) (In%20Cap%20Material :type Material%20Interface%20Object%20Reference) (In%20Procedural%20Mesh :type Procedural%20Mesh%20Component%20Object%20Reference) (In%20Spline%20Component :type Spline%20Component%20Object%20Reference) (In%20Number%20of%20Spline%20sub-divisions :type Integer))
  (bind _triangle_indices (LocalVariables|GetTriangle%20Indices))
  (LocalVariables|SetHeight In%20Height)
  (LocalVariables|SetCap%20Material In%20Cap%20Material)
  (LocalVariables|SetProcedural%20Mesh In%20Procedural%20Mesh)
  (LocalVariables|SetSpline%20Component In%20Spline%20Component)
  (LocalVariables|SetNumber%20of%20Spline%20Sub-divisions In%20Number%20of%20Spline%20sub-divisions)
  (Utilities|Array|Clear (LocalVariables|GetVertex%20Locations%202D))
  ;[1 1 1] Calculate points along the spline to use as vertices
  ;;[1 1 1] For each section of the spline
  (for _index (range 0 (Spline|GetNumberOfSplinePoints (LocalVariables|GetSpline%20Component)))
    (LocalVariables|SetSpline%20Point%20Index _index)
    (for _index_2 (range 0 (LocalVariables|GetNumber%20of%20Spline%20Sub-divisions))
      (Utilities|Array|Add (LocalVariables|GetVertex%20Locations%202D) (Math|Vector2D|MakeVector2D (.x (Spline|GetLocationatTime (LocalVariables|GetSpline%20Component) (|((PointIndex*(1/NumSplinePoints))+(SubIndex*((1/NumSplinePoints)/NumSplineSubdivisions))) (Math|Conversions|ToFloat(Integer) (LocalVariables|GetSpline%20Point%20Index)) (Math|Conversions|ToFloat(Integer) (Spline|GetNumberOfSplinePoints (LocalVariables|GetSpline%20Component))) (Math|Conversions|ToFloat(Integer) _index_2) (Math|Conversions|ToFloat(Integer) (LocalVariables|GetNumber%20of%20Spline%20Sub-divisions))) "Local" false)) (.y (Spline|GetLocationatTime (LocalVariables|GetSpline%20Component) (|((PointIndex*(1/NumSplinePoints))+(SubIndex*((1/NumSplinePoints)/NumSplineSubdivisions))) (Math|Conversions|ToFloat(Integer) (LocalVariables|GetSpline%20Point%20Index)) (Math|Conversions|ToFloat(Integer) (Spline|GetNumberOfSplinePoints (LocalVariables|GetSpline%20Component))) (Math|Conversions|ToFloat(Integer) _index_2) (Math|Conversions|ToFloat(Integer) (LocalVariables|GetNumber%20of%20Spline%20Sub-divisions))) "Local" false))))))
  ;[1 1 1] C++ function uses "Ear clipping" method to find triangles that will represent this polygon well
  (bind _outtris (Class|GeometryBlueprintLibrary|TriangulatePoly (LocalVariables|GetVertex%20Locations%202D) true))
  (Utilities|Array|Clear (LocalVariables|GetProcedural%20Mesh%20Vertices))
  ;[1 1 1] Generate a list of indices into the triangle vertex points to form our triangles
  (for (_array_element _array_index) _outtris
    (Utilities|FlowControl|Sequence
      (:then_0
        ;;[1 1 1] Covert these 2D points to 3D ones, using the specified height
        (Utilities|Array|Add (LocalVariables|GetProcedural%20Mesh%20Vertices) (Math|Vector|MakeVector (.X (Math|Vector2D|BreakVector2D _array_element)) (.Y (Math|Vector2D|BreakVector2D _array_element)) (LocalVariables|GetHeight))))
      (:then_1
        ;;[1 1 1] The triangulate function gives us indices in the order 1,2,3 but the triangles are inverted, so make it 3,2,1 instead
        (if (== (Math|Integer|%(Integer) (+ _array_index 1) 3) 0)
          (Utilities|FlowControl|Sequence
            (:then_0
              (Utilities|Array|SetArrayElem _triangle_indices (- _array_index 2) _array_index true))
            (:then_1
              (Utilities|Array|SetArrayElem _triangle_indices (- _array_index 1) (- _array_index 1) true))
            (:then_2
              (Utilities|Array|SetArrayElem _triangle_indices _array_index (- _array_index 2) true)))))))
  ;[1 1 1] Find min/max points, then map this point's x and y to be in the range 0 to 1
  (bind (_min _max) (CallFunction|FindMinMaxPoints (LocalVariables|GetVertex%20Locations%202D)))
  (LocalVariables|SetMin%20Point _min)
  (LocalVariables|SetMax%20Point _max)
  (for (_array_element_2 _array_index_2) (LocalVariables|GetProcedural%20Mesh%20Vertices)
    (Utilities|Array|SetArrayElem (LocalVariables|GetCap%20UVs) _array_index_2 (Math|Vector2D|MakeVector2D (Math|Float|MapRangeUnclamped (.X (Math|Vector|BreakVector _array_element_2)) (.x (LocalVariables|GetMin%20Point)) (.x (LocalVariables|GetMax%20Point)) 0.0 1.0) (Math|Float|MapRangeUnclamped (.Y (Math|Vector|BreakVector _array_element_2)) (.y (LocalVariables|GetMin%20Point)) (.y (LocalVariables|GetMax%20Point)) 0.0 1.0)) true))
  ;[1 1 1] Create a procedural mesh to represent the top of our wall
  (Class|ProceduralMeshComponent|CreateMeshSection (LocalVariables|GetProcedural%20Mesh) 0 (LocalVariables|GetProcedural%20Mesh%20Vertices) (LocalVariables|GetTriangle%20Indices) 0 (LocalVariables|GetCap%20UVs) 0 0 false)
  ;[1 1 1] Set Material
  (Rendering|Material|SetMaterial (LocalVariables|GetProcedural%20Mesh) 0 (LocalVariables|GetCap%20Material)))

(fn FindMinMaxPoints
  (params (NewParam :type Array%20of%20Vector%202D%20Structures))
  (for _array_element NewParam
    (Utilities|FlowControl|Sequence
      (:then_0
        (Utilities|Array|Add (LocalVariables|GetX%20Values) (.x _array_element)))
      (:then_1
        (Utilities|Array|Add (LocalVariables|GetY%20Values) (.y _array_element)))))
  (return (Math|Vector2D|MakeVector2D (.MinValue (Math|Float|MinOfFloatArray (LocalVariables|GetX%20Values))) (.MinValue (Math|Float|MinOfFloatArray (LocalVariables|GetY%20Values)))) (Math|Vector2D|MakeVector2D (.MaxValue (Math|Float|MaxOfFloatArray (LocalVariables|GetX%20Values))) (.MaxValue (Math|Float|MaxOfFloatArray (LocalVariables|GetY%20Values))))))