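; Player controller for a pinball table, handling flippers, nudging, plunger launch and debug keys for special mode and multiball.
; BeginPlay sorts flippers by side, and input drives each group unless tilted.
; Nudges push every ball sideways with a camera animation, counting per ball until tilt triggers on the game mode and ends ball save.
; Tick builds negative plunger charge while held, and release passes it to the game mode.
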(event EventBeginPlay
  (CallFunction|InitSpecialParts))

(event EventTick
  (params (DeltaSeconds :type Float%20%28single-precision%29))
  (if (Variables|Default|GetChargingPlunger)
    (Utilities|FlowControl|Delay 0.05)
    (Variables|Default|SetShotCharge (Math|Float|Clamp(Float) (+ (Variables|Default|GetShotCharge) -1e+03) -2e+04 0.0))))

(event Input|ActionEvents|InputActionRightFlipper
  (params (Key :type Key%20Structure :default "AnyKey"))
  (bind _flippersright (Variables|Default|GetFlippersRight))
  (:Pressed
    (if (not (Variables|Default|GetTilted))
      (for _array_element _flippersright
        (Default|ActivateFlipper _array_element))))
  (:Released
    (for _array_element_2 _flippersright
      (Default|DeactivateFlipper _array_element_2))))

(event Input|ActionEvents|InputActionLeftFlipper
  (params (Key :type Key%20Structure :default "AnyKey"))
  (bind _flippersleft (Variables|Default|GetFlippersLeft))
  (:Pressed
    (if (not (Variables|Default|GetTilted))
      (for _array_element _flippersleft
        (Default|ActivateFlipper _array_element))))
  (:Released
    (for _array_element_2 _flippersleft
      (Default|DeactivateFlipper _array_element_2))))

(event Input|ActionEvents|InputActionChargePlunger
  (params (Key :type Key%20Structure :default "AnyKey"))
  (:Pressed
    (Variables|Default|SetChargingPlunger (Variables|Default|GetPlungerActive)))
  (:Released
    (if (and (Variables|Default|GetPlungerActive) (< (Variables|Default|GetShotCharge) 0.0))
      (Variables|Default|SetChargingPlunger false)
      (bind _asmy_pinball_game_mode (Utilities|Casting|CastToMyPinballGameMode (Game|GetGameMode)))
      (Default|PlungerShoot _asmy_pinball_game_mode (Variables|Default|GetShotCharge))
      (Variables|Default|SetPlungerActive false)
      (Variables|Default|SetShotCharge 0.0))))

(event Input|ActionEvents|InputActionNudgeRight
  (params (Key :type Key%20Structure :default "AnyKey"))
  ;[1 1 1] Table Nudging
  (:Pressed
    (bind _outactors (Actor|GetAllActorsOfClass "/Game/Blueprints/GamePinball.GamePinball_C"))
    (for _array_element _outactors
      (Physics|AddForce (Variables|/Script/Pinball.PinballBall|GetBall _array_element) "-100000.000000, 0, 0" "None" false)
      (Class|PlayerCameraManager|PlayCameraAnim (Game|GetPlayerCameraManager 0) "/Game/PinballCameraNudge_Right.PinballCameraNudge_Right" 1.0 1.0 0.0 0.0 false false 0.0 "CameraLocal" "0, 0, 0")
      (bind _result (Math|Integer|IncrementInt (Variables|Default|GetNudgeCount))
        (:%20%20
          (if (> _result 3)
            (Variables|Default|SetTilted true)
            (bind _asmy_pinball_game_mode (Utilities|Casting|CastToMyPinballGameMode (Game|GetGameMode)))
            (Default|StartTilt _asmy_pinball_game_mode)
            (Default|EndBallSave _asmy_pinball_game_mode)))))))

(event Input|ActionEvents|InputActionNudgeLeft
  (params (Key :type Key%20Structure :default "AnyKey"))
  ;[1 1 1] Table Nudging
  (:Pressed
    (bind _outactors (Actor|GetAllActorsOfClass "/Game/Blueprints/GamePinball.GamePinball_C"))
    (for _array_element _outactors
      (Physics|AddForce (Variables|/Script/Pinball.PinballBall|GetBall _array_element) "100000.000000, 0, 0" "None" false)
      (Class|PlayerCameraManager|PlayCameraAnim (Game|GetPlayerCameraManager 0) "/Game/PinballCameraNudge_Left.PinballCameraNudge_Left" 1.0 1.0 0.0 0.0 false false 0.0 "CameraLocal" "0, 0, 0")
      (bind _result (Math|Integer|IncrementInt (Variables|Default|GetNudgeCount))
        (:%20%20
          (if (> _result 3)
            (Variables|Default|SetTilted true)
            (bind _asmy_pinball_game_mode (Utilities|Casting|CastToMyPinballGameMode (Game|GetGameMode)))
            (Default|StartTilt _asmy_pinball_game_mode)
            (Default|EndBallSave _asmy_pinball_game_mode)))))))

(event Input|KeyboardEvents|M
  (params (Key :type Key%20Structure :default "AnyKey"))
  (:Pressed
    (bind _asmy_pinball_game_mode (Utilities|Casting|CastToMyPinballGameMode (Game|GetGameMode)))
    (Default|Multiball _asmy_pinball_game_mode)))

(event Input|KeyboardEvents|X
  (params (Key :type Key%20Structure :default "AnyKey"))
  ;[1 1 1] Extra Ball cheat
  (:Pressed
    (Default|StartSpecialMode (Variables|Default|GetSpecialModeComponent) "NewEnumerator3" false)))

(fn ConstructionScript)

(fn InitSpecialParts
  (bind _outactors (Actor|GetAllActorsOfClass "/Game/Blueprints/BP_Flipper.BP_Flipper_C"))
  (for _array_element _outactors
    (switch Utilities|FlowControl|Switch|SwitchonFlipperSide (Variables|/Game/Blueprints/BP_Flipper.BP_Flipper_C|GetFlipperSide _array_element)
      (:NewEnumerator0
        (Utilities|Array|Add (Variables|Default|GetFlippersLeft) _array_element))
      (:NewEnumerator1
        (Utilities|Array|Add (Variables|Default|GetFlippersRight) _array_element)))))

(fn TableNudge
  (params (EndNudge :type Boolean) (LeftNudge :type Boolean))
  (if EndNudge
    (LocalVariables|SetNudgeTime (- (Utilities|Time|GetGameTimeinSeconds) (LocalVariables|GetStartTime)))
    (bind _outactors (Actor|GetAllActorsOfClass "/Game/Blueprints/GamePinball.GamePinball_C"))
    (for _array_element _outactors
      (Physics|AddForce (Variables|/Script/Pinball.PinballBall|GetBall _array_element) (Math|Vector|MakeVector (Math|Float|MapRangeClamped (LocalVariables|GetNudgeTime) 0.0 1.0 -5e+04 -1e+05) 0.0 0.0) "None" false)
      (Class|PlayerCameraManager|PlayCameraAnim (Game|GetPlayerCameraManager 0) "/Game/PinballCameraNudge_Right.PinballCameraNudge_Right" 1.0 1.0 0.0 0.0 false false 0.0 "CameraLocal" "0, 0, 0"))
    (else
      (LocalVariables|SetStartTime (Utilities|Time|GetGameTimeinSeconds)))))