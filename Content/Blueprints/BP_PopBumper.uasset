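; BP_PopBumper is a pinball pop bumper that reacts when a BasePinball overlaps its capsule.
; On hit it plays a sound, registers score and, if FakeIt is set, pushes the ball away from the bumper with an impulse.
; The MechMove timeline drives the mechanism's movement, cap material flash and light intensity together.
; The construction script applies cap texture, flash color and pop speed, with a TestLightup toggle for previewing the lit look.
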(event OnComponentBeginOverlap(Capsule)
  (params (OtherActor :type Actor%20Object%20Reference) (OtherComp :type Primitive%20Component%20Object%20Reference) (OtherBodyIndex :type Integer) (bFromSweep :type Boolean) (SweepResult :type Hit%20Result%20Structure%20%28by%20ref%29))
  (bind _pointlight (Variables|Default|GetPointLight))
  (bind _asbase_pinball (Utilities|Casting|CastToBasePinball OtherActor))
  (Audio|SpawnSoundAttached "/Game/Assets/Audio/Arcade_Enemy_Fire_02_m1.Arcade_Enemy_Fire_02_m1" (Variables|Default|GetSM_PopBumperMechanism))
  (if (Variables|PopBumper|GetFakeIt)
    (Physics|AddImpulse (Variables|/Script/Pinball.PinballBall|GetBall _asbase_pinball) (* (Math|Vector|Normalize (- (Transformation|GetActorLocation _asbase_pinball) (+ (Transformation|GetActorLocation) "0, 0,50.000000"))) (Variables|PopBumper|GetImpulsePower)) "None" false))
  (Default|RegisterScore (Variables|Default|GetScoreComponent))
  (Rendering|SetVisibility _pointlight true false)
  (bind _newtrack_0 (Timeline|MechMove PlayFromStart)
    (:Update
      (Transformation|SetRelativeLocation (Variables|Default|GetSM_PopBumperMechanism) (Math|Vector|Lerp(Vector) "0, 0,20.000000" "0, 0,-70.000000" _newtrack_0) false false)
      (Rendering|Material|SetScalarParameterValue (Variables|PopBumper|GetCapMat) "Flash" _newtrack_0 :!class /Script/Engine.MaterialInstanceDynamic)
      (Rendering|Components|Light|SetIntensity (Variables|Default|GetPointLight) (* _newtrack_0 5e+04)))
    (:Finished
      (Rendering|SetVisibility _pointlight false false))))

(event EventBeginPlay)

(event Collision|EventActorBeginOverlap
  (params (OtherActor :type Actor%20Object%20Reference)))

(event EventTick
  (params (DeltaSeconds :type Float%20%28single-precision%29)))

(fn ConstructionScript
  (bind _flashcolor (Variables|PopBumper|GetFlashColor))
  (bind _returnvalue (Rendering|Material|CreateDynamicMaterialInstance (Variables|Default|GetSM_PopBumperBase) 1 (Variables|PopBumper|GetBumperCapMaterial) :!class /Script/Engine.PrimitiveComponent))
  (bind _output_get (Variables|PopBumper|SetCapMat _returnvalue))
  (Rendering|Material|SetTextureParameterValue _output_get "CapTexture" (Variables|PopBumper|GetBumperCapTexture))
  (Rendering|Material|SetVectorParameterValue _output_get "FlashColor" _flashcolor :!class /Script/Engine.MaterialInstanceDynamic)
  (Rendering|Components|Light|SetLightColor (Variables|Default|GetPointLight) _flashcolor true)
  (Utilities|FlowControl|Sequence
    (:then_0
      ;[1 1 1] Temporarily Turn on Light and Mat Color to check color
      (if (Variables|PopBumper|GetTestLightup)
        (Rendering|Material|SetScalarParameterValue (Variables|PopBumper|GetCapMat) "Flash" 1.0 :!class /Script/Engine.MaterialInstanceDynamic)
        (Rendering|Components|Light|SetIntensity (Variables|Default|GetPointLight) 5e+04)))
    (:then_1
      (Components|Timeline|SetPlayRate (Variables|Default|GetMechMove) (Variables|PopBumper|GetPopSpeedMultiplier)))))