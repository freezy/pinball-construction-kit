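; BP_Flipper is a pinball flipper that swings between a start and end yaw when activated and released.
; Activate plays an attached sound and uses MoveComponentTo to rotate the mesh over FlipperRotationTime; Deactivate clears the held flag and rotates it back.
; The construction script sets the rest pose, points an arrow at the end angle and colors body and rubber through dynamic materials.
; An older RotationLerp timeline path remains but never runs.
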(event Custom|DeactivateFlipper
  (Variables|Flipper|SetFlipperHeld false)
  (CallFunction|ReturnFlipper))

(event Custom|ReturnFlipper
  (Components|MoveComponentTo (Variables|Default|GetFlipperMesh) "0, 0, 0" (Math|Rotator|MakeRotator 0.0 0.0 (Variables|Flipper|GetStartRotation)) false false (Variables|Flipper|GetFlipperRotationTime)))

(event Custom|ActivateFlipper
  (Audio|SpawnSoundAttached "/Game/Sounds/Pinball_FlipperLeft.Pinball_FlipperLeft" (Variables|Default|GetFlipperMesh) "None" "0, 0, 0" "0, 0, 0" "SnapToTargetIncludingScale" false 0.5)
  (Variables|Flipper|SetFlipperHeld true)
  (Components|MoveComponentTo (Variables|Default|GetFlipperMesh) "0, 0, 0" (Math|Rotator|MakeRotator 0.0 0.0 (Variables|Flipper|GetEndRotation)) false false (Variables|Flipper|GetFlipperRotationTime)))

(event EventBeginPlay)

(event EventActorBeginOverlap
  (params (OtherActor :type Actor%20Object%20Reference)))

(event EventTick
  (params (DeltaSeconds :type Float%20%28single-precision%29)))

(fn ConstructionScript
  (bind _flippermesh (Variables|Default|GetFlipperMesh))
  (Components|Timeline|SetPlayRate (Variables|Default|GetRotationLerp) (/ 1.0 (Variables|Flipper|GetFlipperRotationTime)))
  (Transformation|SetRelativeRotation (Variables|Default|GetFlipperMesh) (Math|Rotator|MakeRotator 0.0 0.0 (Variables|Flipper|GetStartRotation)) false false)
  (Transformation|SetRelativeRotation (Variables|Default|GetArrow) (Math|Rotator|MakeRotator 0.0 0.0 (Variables|Flipper|GetEndRotation)) false false)
  (bind _returnvalue (Rendering|Material|CreateDynamicMaterialInstance _flippermesh 0 0 :!class /Script/Engine.PrimitiveComponent))
  (bind _returnvalue_2 (Rendering|Material|CreateDynamicMaterialInstance _flippermesh 1 0 :!class /Script/Engine.PrimitiveComponent))
  (Rendering|Material|SetVectorParameterValue _returnvalue "BaseColor" (Variables|Flipper|GetFlipperColor) :!class /Script/Engine.MaterialInstanceDynamic)
  (Rendering|Material|SetVectorParameterValue _returnvalue_2 "BaseColor" (Variables|Flipper|GetRubberColor) :!class /Script/Engine.MaterialInstanceDynamic))