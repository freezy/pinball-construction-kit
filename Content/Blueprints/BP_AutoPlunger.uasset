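; Pinball auto-plunger actor that fires when a ball overlaps its trigger, up to a limited number of saves.
; The overlap, ignored while the player controller is tilted, passes a DoOnce gate, plays a sound and runs a timeline that slides the plunger along relative Y.
; The timeline's end re-arms the gate while uses remain.
; ReinitPlunger clears the count and re-arms it if per-ball reset is enabled.
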(event OnComponentBeginOverlap(Trigger)
  (params (OtherActor :type Actor%20Object%20Reference) (OtherComp :type Primitive%20Component%20Object%20Reference) (OtherBodyIndex :type Integer) (bFromSweep :type Boolean) (SweepResult :type Hit%20Result%20Structure%20%28by%20ref%29))
  (Utilities|Casting|CastToBasePinball OtherActor)
  (bind _aspinball_player_controller (Utilities|Casting|CastToPinballPlayerController (Game|GetPlayerController 0))) ; do nothing when tilted
  (if (not (Variables|/Game/Blueprints/PinballPlayerController.PinballPlayerController_C|GetTilted _aspinball_player_controller))
    (Utilities|FlowControl|DoOnce false
      (:Completed
        (Math|Integer|IncrementInt (Variables|Default|GetUseCount)
          (:%20%20
            (Audio|PlaySoundatLocation "/Game/Assets/Audio/Arcade_Enemy_Death_01_m1.Arcade_Enemy_Death_01_m1" (Transformation|GetActorLocation))
            (bind _alpha (Timeline|Movement PlayFromStart)
              (:Update
                (Transformation|SetRelativeLocation (Variables|Default|Getplunger) (Math|Vector|MakeVector 0.0 (Math|Float|Lerp 3.8e+02 0.0 _alpha) 5e+01) false false))
              (:Finished
                (if (< (Variables|Default|GetUseCount) (Variables|AutoPlunger|GetNumberOfSaves))
                  (CallFunction|ResetPlunger))))))))))

(event Custom|ReinitPlunger
  ;[1 1 1] GameMode can reset count for each for each ball
  (if (Variables|AutoPlunger|GetResetPerBall)
    (Variables|Default|SetUseCount 0)
    (CallFunction|ResetPlunger)))

(event Custom|ResetPlunger
  (Utilities|FlowControl|DoOnce false) ; enters at Reset
)

(event EventBeginPlay)

(event EventActorBeginOverlap
  (params (OtherActor :type Actor%20Object%20Reference)))

(event EventTick
  (params (DeltaSeconds :type Float%20%28single-precision%29)))

(fn ConstructionScript)