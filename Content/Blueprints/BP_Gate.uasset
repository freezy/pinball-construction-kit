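; BP_Gate is a pinball gate: a physics tile between two brackets that scores when a ball knocks it spinning.
; A BasePinball hit waits briefly, then registers score through ScoreComponent if the tile's angular velocity is high enough.
; The construction script builds the gate parametrically from an end point, bracket height, clearance and tile width, placing, scaling and aiming the brackets, rod, constraint and tile.
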(event OnComponentHit(Tile)
  (params (OtherActor :type Actor%20Object%20Reference) (OtherComp :type Primitive%20Component%20Object%20Reference) (NormalImpulse :type Vector :default "0, 0, 0") (Hit :type Hit%20Result%20Structure%20%28by%20ref%29))
  (Utilities|Casting|CastToBasePinball OtherActor)
  (Utilities|FlowControl|Delay 0.2)
  (bind _returnvalue (Class|PrimitiveComponent|GetPhysicsAngularVelocity (Variables|Default|GetTile) "None"))
  (if (>= (Math|Vector|VectorLength _returnvalue) 45.0)
    (Default|RegisterScore (Variables|Default|GetScoreComponent))))

(event EventBeginPlay)

(event Collision|EventActorBeginOverlap
  (params (OtherActor :type Actor%20Object%20Reference)))

(event EventTick
  (params (DeltaSeconds :type Float%20%28single-precision%29)))

(fn ConstructionScript
  (bind _returnvalue (Math|Vector|MakeVector 0.0 0.0 0.0))
  (bind _bracketendpoint (Variables|Default|GetBracketEndPoint))
  (bind _bracketendpoint_2 (Variables|Default|GetBracketEndPoint))
  (bind _bracketendpoint_3 (Variables|Default|GetBracketEndPoint))
  (bind _bracketheight (Variables|Default|GetBracketHeight))
  (bind _tile (Variables|Default|GetTile))
  (bind _gateclearanceheight (Variables|Default|GetGateClearanceHeight))
  (bind _bracketheight_2 (Variables|Default|GetBracketHeight))
  (bind _returnvalue_2 (- 75.0 _bracketheight_2))
  (bind _returnvalue_3 (- _returnvalue _bracketendpoint_2))
  (bind _returnvalue_4 (Math|Vector|VectorLength _returnvalue_3))
  (bind _returnvalue_5 (+ _returnvalue_2 _gateclearanceheight))
  (bind _returnvalue_6 (+ _returnvalue_5 5e+01))
  (Transformation|SetRelativeLocation (Variables|Default|GetRotateroot) (Math|Vector|MakeVector 0.0 0.0 _bracketheight) false false)
  (Transformation|SetRelativeLocation (Variables|Default|Get2ndBracket) (Math|Vector|MakeVector (.x _bracketendpoint) (.y _bracketendpoint) _bracketheight) false false)
  (Transformation|SetRelativeLocation (Variables|Default|GetPhysicsConstraint) (Math|Vector|MakeVector 2e+01 0.0 _returnvalue_6) false false)
  (Transformation|SetRelativeScale3D (Variables|Default|GetSM_BracketTop) (Math|Vector|MakeVector (/ (- _returnvalue_4 4e+01) 1e+02) 1.0 1.0))
  (Transformation|SetRelativeLocation _tile (Math|Vector|MakeVector (/ _returnvalue_4 2.0) 0.0 _returnvalue_5) false false)
  (Transformation|SetRelativeScale3D _tile (Math|Vector|MakeVector (Variables|Default|GetTileWidthMultiplier) 1.0 1.0))
  (Transformation|SetRelativeRotation (Variables|Default|GetRotateroot) (Math|Rotator|FindLookatRotation _returnvalue _bracketendpoint_3) false false)
  (Transformation|SetRelativeRotation (Variables|Default|Get2ndBracket) (Math|Rotator|FindLookatRotation _bracketendpoint_3 _returnvalue) false false)
  (Transformation|SetRelativeScale3D (Variables|Default|GetSM_LBracket) (Math|Vector|MakeVector 1.0 1.0 (/ (+ _returnvalue_6 5e+01) 1e+02))))