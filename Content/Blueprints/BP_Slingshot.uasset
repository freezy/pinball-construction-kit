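; BP_Slingshot is a pinball slingshot bumper that kicks the ball away when it hits the rubber band's capsule trigger.
; On overlap it applies an impulse from Center toward the Direction component, weakened as the ball lands farther from the center.
; It also plays a bump sound, registers score through ScoreComponent, and flexes the band's morph target with a timeline.
; A FlipX option in the construction script mirrors the mesh and trigger for the opposite side.
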(event OnComponentBeginOverlap(CapsuleTrigger)
  (params (OtherActor :type Actor%20Object%20Reference) (OtherComp :type Primitive%20Component%20Object%20Reference) (OtherBodyIndex :type Integer) (bFromSweep :type Boolean) (SweepResult :type Hit%20Result%20Structure%20%28by%20ref%29))
  (bind _center (Variables|Default|Getcenter))
  (bind _returnvalue (Transformation|GetWorldLocation _center))
  (bind _asbase_pinball (Utilities|Casting|CastToBasePinball OtherActor))
  (Physics|AddImpulse (Variables|/Script/Pinball.PinballBall|GetBall _asbase_pinball) (* (Math|Vector|Normalize (- (Transformation|GetWorldLocation (Variables|Default|Getdirection)) _returnvalue)) (* (Variables|Default|GetPower) (Math|Float|MapRangeClamped (Math|Vector|VectorLength (- (Transformation|GetWorldLocation (Variables|/Script/Pinball.PinballBall|GetBall _asbase_pinball)) _returnvalue)) 2e+02 2.5e+02 1.0 0.3))) "None" false)
  (Audio|PlaySoundatLocation "/Game/Sounds/SlingshotBump.SlingshotBump" (Transformation|GetActorLocation) "0, 0, 0" 0.8)
  (Default|RegisterScore (Variables|Default|GetScoreComponent))
  (bind _alpha (Timeline|BandFlex PlayFromStart)
    (:Update
      (Components|SkeletalMesh|SetMorphTarget (Variables|Default|GetRubberBand) "Slingband_morph" _alpha false))))

(event EventBeginPlay)

(event Collision|EventActorBeginOverlap
  (params (OtherActor :type Actor%20Object%20Reference)))

(event EventTick
  (params (DeltaSeconds :type Float%20%28single-precision%29)))

(fn ConstructionScript
  (if (Variables|Default|GetFlipX)
    (Transformation|SetRelativeScale3D (Variables|Default|GetReverse) "-1.000000,1.000000,1.000000")
    (Transformation|SetRelativeRotation (Variables|Default|GetCapsuleTrigger) "0,-20.000000,-90.000000" false false)))