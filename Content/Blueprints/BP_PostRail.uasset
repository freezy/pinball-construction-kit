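; BP_PostRail is a configurable rail of two posts joined by a rubber band, with tintable materials and two point lights.
; The construction script creates shared dynamic materials for post and rubber colors, sets the light color, then calls AdjustBandSize.
; AdjustBandSize places EndPost at EndPostLocation's X/Y, scales the band extender to the span and turns both posts to face each other.
; It has no active runtime logic.
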(event EventBeginPlay)

(event Collision|EventActorBeginOverlap
  (params (OtherActor :type Actor%20Object%20Reference)))

(event EventTick
  (params (DeltaSeconds :type Float%20%28single-precision%29)))

(fn ConstructionScript
  (bind _returnvalue (Rendering|Material|CreateDynamicMaterialInstance (Variables|Default|GetStaticMesh) 0 0 :!class /Script/Engine.PrimitiveComponent))
  (Rendering|Material|SetMaterial (Variables|Default|GetEndPost) 0 _returnvalue)
  (Rendering|Material|SetVectorParameterValue _returnvalue "BaseColor" (Variables|Default|GetPostColor) :!class /Script/Engine.MaterialInstanceDynamic)
  (Rendering|Components|Light|SetLightColor (Variables|Default|GetPointLight) (Variables|Default|GetLightColor) true)
  (bind _returnvalue_2 (Rendering|Material|CreateDynamicMaterialInstance (Variables|Default|GetStaticMesh) 1 0 :!class /Script/Engine.PrimitiveComponent))
  (Rendering|Material|SetVectorParameterValue _returnvalue_2 "BaseColor" (Variables|Default|GetRubberColor) :!class /Script/Engine.MaterialInstanceDynamic)
  (Rendering|Material|SetMaterial (Variables|Default|GetEndPost) 1 _returnvalue_2)
  (CallFunction|AdjustBandSize))

(fn AdjustBandSize
  (bind _returnvalue (Math|Vector|MakeVector 0.0 0.0 0.0))
  (bind _endpostlocation (Variables|Default|GetEndPostLocation))
  (bind _endpostlocation_2 (Variables|Default|GetEndPostLocation))
  (Transformation|SetRelativeLocation (Variables|Default|GetEndPost) (Math|Vector|MakeVector (.x _endpostlocation) (.y _endpostlocation) 0.0) false false)
  (Transformation|SetRelativeScale3D (Variables|Default|GetSM_BandExtender) (Math|Vector|MakeVector (/ (Math|Vector|VectorLength (- _returnvalue _endpostlocation_2)) 1e+02) 1.0 1.0))
  (Transformation|SetRelativeRotation (Variables|Default|GetStaticMesh) (Math|Rotator|FindLookatRotation _returnvalue _endpostlocation_2) false false)
  (Transformation|SetRelativeRotation (Variables|Default|GetEndPost) (Math|Rotator|FindLookatRotation _endpostlocation_2 _returnvalue) false false))