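; BP_TargetSet builds a configurable row of BP_DropTarget child actors that report hits to a target controller and can be reset together.
; The construction script spawns evenly spaced targets, applies per-target style data and a shared score, optionally copies the first target's colors to all, and collects objects to activate.
; At BeginPlay it indexes and binds each target, forwarding hits to the controller or warning if none is assigned.
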(event Custom|TargetHit_Event_0
  (params (TargetIndex :type Integer))
  (bind _mytargetcontroller (Variables|Default|GetMyTargetController))
  (Utilities|IsValid _mytargetcontroller
    (:Is%20Valid
      (Default|NotifyTargetDowned _mytargetcontroller))
    (:Is%20Not%20Valid
      (Development|PrintString (Utilities|String|BuildString(Object) "" "WARNING: " self "has no Target Controller Assigned")))))

(event Custom|Resettargets
  (for _array_element (Variables|Default|GetTargets)
    (bind _asbp_drop_target (Utilities|Casting|CastToBP_DropTarget (Variables|/Script/Engine.ChildActorComponent|GetChildActor _array_element)))
    (Default|Reset _asbp_drop_target)))

(event EventBeginPlay
  (for (_array_element _array_index) (Variables|Default|GetTargets)
    (bind _asbp_drop_target (Utilities|Casting|CastToBP_DropTarget (Variables|/Script/Engine.ChildActorComponent|GetChildActor _array_element)))
    (Variables|/Game/Blueprints/BP_DropTarget.BP_DropTarget_C|SetTargetIndex _asbp_drop_target _array_index)
    (EventDispatchers|AssignTargetHit _asbp_drop_target (delegate Custom|TargetHit_Event_0))))

(event Collision|EventActorBeginOverlap
  (params (OtherActor :type Actor%20Object%20Reference)))

(event EventTick
  (params (DeltaSeconds :type Float%20%28single-precision%29)))

(fn ConstructionScript
  (Utilities|Array|Clear (Variables|Default|GetTargets))
  (for _index (range 0 (- (Variables|DropTargetSet|GetNumberOfTargets) 1))
    (bind _returnvalue (AddComponent|AddChildActorComponent false (Math|Transform|MakeTransform (Math|Vector|MakeVector (Math|Conversions|ToFloat(Integer) (* _index 120)) 0.0 0.0) "0, 0, 0" "1,1,1")))
    (Utilities|Array|Add (Variables|Default|GetTargets) _returnvalue)
    (Utilities|Array|Resize (Variables|DropTargetSet|GetTargetData) (Variables|DropTargetSet|GetNumberOfTargets))
    (Utilities|Array|Clear (Variables|Default|GetObjectsToActivate))
    (if (Variables|DropTargetSet|GetUnitfy%20Colors)
      (for (_array_element _array_index) (Variables|DropTargetSet|GetTargetData)
        (Utilities|Array|SetArrayElem (Variables|DropTargetSet|GetTargetData) _array_index (Utilities|Struct|MakeDropTargetStruct (.targetstyle _array_element) (.droptargettexture _array_element) (.basecolor (Utilities|Array|Get(acopy) (Variables|DropTargetSet|GetTargetData))) (.targetcolor (Utilities|Array|Get(acopy) (Variables|DropTargetSet|GetTargetData))) (.lettercolor (Utilities|Array|Get(acopy) (Variables|DropTargetSet|GetTargetData))) (.objecttoactivate _array_element)))))
    (for (_array_element_2 _array_index_2) (Variables|DropTargetSet|GetTargetData)
      (Utilities|Array|Add (Variables|Default|GetObjectsToActivate) (.ObjectToActivate (Utilities|Struct|BreakDropTargetStruct _array_element_2)))
      (bind _asbp_drop_target (Utilities|Casting|CastToBP_DropTarget (Variables|/Script/Engine.ChildActorComponent|GetChildActor (Utilities|Array|Get(acopy) (Variables|Default|GetTargets) _array_index_2))))
      (Variables|/Game/Blueprints/BP_DropTarget.BP_DropTarget_C|SetTargetData _asbp_drop_target _array_element_2)
      (Variables|/Game/Components/ScoreComponent.ScoreComponent_C|SetPointValue (Variables|/Game/Blueprints/BP_DropTarget.BP_DropTarget_C|GetScoreComponent _asbp_drop_target) (Variables|DropTargetSet|GetTargetScoreValue))
      (Default|SetTargetStyle _asbp_drop_target))))