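; Spline-based ramp actor, built entirely in the Construction Script, that can turn into a rail over its final sections.
; It optionally resets to a straight default spline, then slopes point heights over the first SlopeSectionCount sections.
; A shared helper creates spline meshes, then AddRail swaps trailing segments to rail meshes and adds rings at their points.
; An optional end cap follows, and ScaleRamp tapers width and applies wall height.
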(event EventBeginPlay)

(event EventActorBeginOverlap
  (params (OtherActor :type Actor%20Object%20Reference)))

(event EventTick
  (params (DeltaSeconds :type Float%20%28single-precision%29)))

(fn ConstructionScript
  (bind _splinemeshcomponents (Variables|Default|GetSplineMeshComponents))
  (if (Variables|Default|GetbResetSplineToDefault)
    (CallFunction|CreateDefaultSpline))
  (CallFunction|SetSlope)
  (Utilities|Array|SetArrayElem (Variables|Default|GetSideMaterials) 0 (Variables|Ramp|GetRampMaterial) true)
  (bind _outsidematerials (CallFunction|AddSplineMeshComponents (Variables|Default|GetSplineComponent) self 1e+02 (Variables|Default|GetSideMaterials) (Variables|Default|GetNumberTextures) (Variables|Ramp|GetRampMesh) true))
  (Variables|Default|SetSideMaterials _outsidematerials)
  (CallFunction|AddRail)
  (if (Variables|Ramp|GetCapEnd)
    (Components|StaticMesh|SetStaticMesh (Utilities|Array|Get(acopy) _splinemeshcomponents (Utilities|Array|LastIndex _splinemeshcomponents)) "/Game/Meshes/SM_PlasticRamp_End.SM_PlasticRamp_End"))
  (CallFunction|ScaleRamp))

(fn ScaleRamp
  (bind _splinecomponent (Variables|Default|GetSplineComponent))
  (LocalVariables|SetEndLength (select (> (Variables|Rail|GetRailSectionCount) 0) (Spline|GetDistanceAlongSplineatSplinePoint _splinecomponent (- (Spline|GetNumberOfSplinePoints _splinecomponent) (Variables|Rail|GetRailSectionCount))) (Spline|GetSplineLength (Variables|Default|GetSplineComponent))))
  (for (_array_element _array_index) (Variables|Default|GetSplineMeshComponents)
    (bind _output_get (LocalVariables|SetStartIndex _array_index))
    (LocalVariables|SetEndIndex (+ _output_get 1))
    (SplineMesh|SetStartScale _array_element (Math|Vector2D|MakeVector2D (Math|Float|Lerp (Variables|Ramp|GetStartWidth) (Variables|Ramp|GetEndWidth) (Math|Float|Clamp(Float) (/ (Spline|GetDistanceAlongSplineatSplinePoint (Variables|Default|GetSplineComponent) (LocalVariables|GetStartIndex)) (LocalVariables|GetEndLength)))) (Variables|Ramp|GetWallHeight)) :!class /Script/Engine.SplineMeshComponent)
    (SplineMesh|SetEndScale _array_element (Math|Vector2D|MakeVector2D (Math|Float|Lerp (Variables|Ramp|GetStartWidth) (Variables|Ramp|GetEndWidth) (Math|Float|Clamp(Float) (/ (Spline|GetDistanceAlongSplineatSplinePoint (Variables|Default|GetSplineComponent) (LocalVariables|GetEndIndex)) (LocalVariables|GetEndLength)))) (Variables|Ramp|GetWallHeight)) :!class /Script/Engine.SplineMeshComponent)))

(fn SetSlope
  (bind _splinecomponent (Variables|Default|GetSplineComponent))
  (bind _splinecomponent_2 (Variables|Default|GetSplineComponent))
  (bind _splinecomponent_3 (Variables|Default|GetSplineComponent))
  (bind _meshlipadjustment (Variables|Ramp|GetMeshLipAdjustment))
  (LocalVariables|SetRampLength (Spline|GetDistanceAlongSplineatSplinePoint _splinecomponent_3 (Math|Integer|Min(Integer) (Variables|Ramp|GetSlopeSectionCount) (- (Spline|GetNumberOfSplinePoints _splinecomponent_3) 1))))
  (for _index (range 0 (- (Spline|GetNumberOfSplinePoints _splinecomponent) 1))
    (Spline|SetLocationatSplinePoint _splinecomponent_2 _index (Math|Vector|MakeVector (.x (Spline|GetLocationatSplinePoint _splinecomponent_2 _index "Local")) (.y (Spline|GetLocationatSplinePoint _splinecomponent_2 _index "Local")) (Math|Float|Lerp (+ (Variables|Ramp|GetStartHeight) _meshlipadjustment) (+ _meshlipadjustment (Variables|Ramp|GetEndHeight)) (Math|Float|Clamp(Float) (/ (Spline|GetDistanceAlongSplineatSplinePoint _splinecomponent _index) (LocalVariables|GetRampLength))))) "Local")))

(fn CreateDefaultSpline
  (bind _splinecomponent (Variables|Default|GetSplineComponent))
  (Spline|ClearSplinePoints _splinecomponent)
  (for _index (range 0 4)
    (Spline|AddSplinePoint _splinecomponent (Math|Vector|MakeVector 0.0 (* _index (* (/ (Variables|Ramp|GetDefaultLength) 4.0) -1.0)) 0.0) "Local")))

(fn AddRail
  (bind _splinecomponent (Variables|Default|GetSplineComponent))
  (bind _splinemeshcomponents (Variables|Default|GetSplineMeshComponents))
  (bind _splinecomponent_2 (Variables|Default|GetSplineComponent))
  (bind _railsectioncount (Variables|Rail|GetRailSectionCount))
  (bind _railsectioncount_2 (Variables|Rail|GetRailSectionCount))
  (bind _returnvalue (Spline|GetNumberOfSplinePoints _splinecomponent_2))
  (bind _returnvalue_2 (Spline|GetNumberOfSplinePoints _splinecomponent))
  (bind _returnvalue_3 (- _returnvalue 1))
  (bind _returnvalue_4 (- _returnvalue_3 _railsectioncount_2))
  (bind _item (Utilities|Array|Get(acopy) _splinemeshcomponents _returnvalue_4))
  (Components|StaticMesh|SetStaticMesh _item "/Game/Meshes/SM_RailMouth.SM_RailMouth")
  (Rendering|Material|SetMaterial _item 0 (Variables|Rail|GetRailMaterial))
  (for _index (range (+ _returnvalue_4 1) _returnvalue_3)
    (Components|StaticMesh|SetStaticMesh (Utilities|Array|Get(acopy) (Variables|Default|GetSplineMeshComponents) _index) (select (== _index (- _returnvalue_3 1)) "/Game/Meshes/SM_RailEnd.SM_RailEnd" (Variables|Rail|GetRailMesh)))
    (Rendering|Material|SetMaterial (Utilities|Array|Get(acopy) (Variables|Default|GetSplineMeshComponents) _index) 0 (Variables|Rail|GetRailMaterial)))
  (if (> _railsectioncount 0)
    ;[1 1 1] Add Rings
    (for _index_2 (range (- _returnvalue_2 _railsectioncount) _returnvalue_2)
      (AddComponent|AddStaticMeshComponent false (Math|Transform|MakeTransform (Spline|GetLocationatSplinePoint _splinecomponent _index_2 "Local") (Spline|GetRotationatSplinePoint _splinecomponent _index_2 "Local") (Math|Vector|MakeVector 1.0 1.0 (Variables|Ramp|GetWallHeight)))))))