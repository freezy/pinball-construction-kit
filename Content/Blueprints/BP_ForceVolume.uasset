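; BP_ForceVolume is a trigger volume for pinball, apparently meant to push a ball that enters it.
; The construction script sizes the Box as a cube, using the distance from the actor to Bounds as each extent.
; On overlap, it stores the GamePinball and sets ForceOn, which nothing here clears or reads.
; The negative-X AddForce on the ball is disconnected and Tick is empty, so no force is applied here.
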(event OnComponentBeginOverlap(Box)
  (params (OtherActor :type Actor%20Object%20Reference) (OtherComp :type Primitive%20Component%20Object%20Reference) (OtherBodyIndex :type Integer) (bFromSweep :type Boolean) (SweepResult :type Hit%20Result%20Structure%20%28by%20ref%29))
  (bind _asgame_pinball (Utilities|Casting|CastToGamePinball OtherActor))
  (Variables|Default|SetPinball _asgame_pinball)
  (Variables|Default|SetForceOn true))

(event EventBeginPlay)

(event Collision|EventActorBeginOverlap
  (params (OtherActor :type Actor%20Object%20Reference)))

(event EventTick
  (params (DeltaSeconds :type Float%20%28single-precision%29)))

(fn ConstructionScript
  (bind _returnvalue (Transformation|GetActorLocation))
  (bind _bounds (Variables|Default|GetBounds))
  (bind _returnvalue_2 (- _bounds _returnvalue))
  (bind _returnvalue_3 (Math|Vector|VectorLength _returnvalue_2))
  (Components|Box|SetBoxExtent (Variables|Default|GetBox) (Math|Vector|MakeVector _returnvalue_3 _returnvalue_3 _returnvalue_3) true))