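; GamePinball is the pinball actor, simulating the pull of a sloped table on its Ball component.
; Each tick, unless BallTrapped is set, it applies a frame-time-scaled velocity-change impulse along +Y to roll the ball down the table.
; It also traces downward and pushes the ball against the hit surface normal by TableStickyForce to limit popping up.
; A separate AddTrail event activates the particle system.
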(event Custom|AddTrail
  (Components|Activation|Activate (Variables|Default|GetParticleSystem) false))

(event EventBeginPlay)

(event EventActorBeginOverlap
  (params (OtherActor :type Actor%20Object%20Reference)))

(event EventTick
  (params (DeltaSeconds :type Float%20%28single-precision%29))
  (bind _returnvalue (Transformation|GetActorLocation))
  ;[1 1 1] Apply constant force "down" the table
  (if (not (Variables|Default|GetBallTrapped)) ; Stop force when ball is trapped
    (Physics|AddImpulse (Variables|Default|GetBall) (Math|Vector|MakeVector 0.0 (* DeltaSeconds 2075.0) 0.0) "None" true)
    ;[1 1 1] A bit of force toward the surface to keep the ball from popping up too much
    (bind _outhit (Collision|LineTraceByChannel _returnvalue (- _returnvalue "0, 0,300.000000") "TraceTypeQuery1" false 0 "None"))
    (Physics|AddImpulse (Variables|Default|GetBall) (* (* (.ImpactNormal (Collision|BreakHitResult _outhit)) -1.0) (* DeltaSeconds (Variables|Default|GetTableStickyForce))) "None" true)))

(fn ConstructionScript
  (|CallParentFunction))