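; BP_Indicator_Rollover is a pinball rollover indicator that a ball toggles by rolling over it.
; When a BasePinball enters its trigger, it plays an activation sound and alternates through a FlipFlop between on and off states.
; Turning on activates itself, messages its linked ObjectToActivate and registers score through its ScoreComponent, while turning off deactivates both without scoring.
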(event OnComponentBeginOverlap(Trigger)
  (params (OtherActor :type Actor%20Object%20Reference) (OtherComp :type Primitive%20Component%20Object%20Reference) (OtherBodyIndex :type Integer) (bFromSweep :type Boolean) (SweepResult :type Hit%20Result%20Structure%20%28by%20ref%29))
  (bind _objecttoactivate (Variables|Default|GetObjectToActivate))
  ;[1 1 1] When ball rolls over, turn light on/off and activate/deactivate relevant object. Add to score if any
  (Utilities|Casting|CastToBasePinball OtherActor)
  (Audio|PlaySoundatLocation (Variables|Default|GetActivationSound) (Transformation|GetActorLocation))
  (Utilities|FlowControl|FlipFlop
    (:A
      (CallFunction|Activate)
      (Class|PinballInterface|Activate(Message) _objecttoactivate)
      (Default|RegisterScore (Variables|Default|GetScoreComponent)))
    (:B
      (CallFunction|Deactivate)
      (Class|PinballInterface|Deactivate(Message) _objecttoactivate))))

(event EventBeginPlay
  (|CallParentFunction))

(event EventActorBeginOverlap
  (params (OtherActor :type Actor%20Object%20Reference)))

(event EventTick
  (params (DeltaSeconds :type Float%20%28single-precision%29)))

(fn ConstructionScript
  (|CallParentFunction))