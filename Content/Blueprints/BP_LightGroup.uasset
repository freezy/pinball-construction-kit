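; BP_LightGroup tracks a set of lights and rewards the player once all of them are lit.
; On BeginPlay it registers itself with each light, and NotifyLitUnlit maintains a count of lit ones.
; A full count registers score, starts a special mode and, after a short delay, plays an ordered-on sequence followed by a group flash.
; The lighttest event triggers that light sequence directly.
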(event Custom|lighttest
  (bind _lights (Variables|Default|GetLights))
  (Utilities|Orderedon _lights 0.2
    (:Complete
      (Utilities|AllFlash _lights 2 0.2))))

(event Custom|NotifyLitUnlit
  (params (Lit :type Boolean))
  (bind _lights (Variables|Default|GetLights))
  (if Lit
    (Math|Integer|IncrementInt (Variables|Default|GetLitLights)
      (:%20%20
        (if (== (Variables|Default|GetLitLights) (Utilities|Array|Length (Variables|Default|GetLights)))
          (Default|RegisterScore (Variables|Default|GetScoreComponent))
          (Default|StartSpecialMode (Variables|Default|GetSpecialModeComponent) "NewEnumerator0" false)
          (Utilities|FlowControl|Delay 0.2)
          (Utilities|Orderedon _lights 0.2
            (:Complete
              (Utilities|AllFlash _lights 2 0.2))))))
    (else
      (Math|Integer|DecrementInt (Variables|Default|GetLitLights)))))

(event EventBeginPlay
  ;[1 1 1] tell each light that it's part of this group
  (for _array_element (Variables|Default|GetLights)
    (Variables|/Game/Blueprints/BP_IndicatorLight.BP_IndicatorLight_C|SetMyLightGroup _array_element self)))

(event EventActorBeginOverlap
  (params (OtherActor :type Actor%20Object%20Reference)))

(event EventTick
  (params (DeltaSeconds :type Float%20%28single-precision%29)))

(fn ConstructionScript)