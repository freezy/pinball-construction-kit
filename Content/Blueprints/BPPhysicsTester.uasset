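; BPPhysicsTester is a pinball physics test rig: a tilted table with a ball spawn, plunger and end wall.
; BeginPlay spawns a BasePinball and targets it with damping and material setup; construction sets table tilt and plunger speed.
; A bottom box overlap fires a gated timeline that lerps the plunger out, then reverses and reopens the gate.
; Bottom and end wall contact times are recorded, with end wall hit times printed.
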(event OnComponentHit(EndWall)
  (params (OtherActor :type Actor%20Object%20Reference) (OtherComp :type Primitive%20Component%20Object%20Reference) (NormalImpulse :type Vector :default "0, 0, 0") (Hit :type Hit%20Result%20Structure%20%28by%20ref%29))
  (bind _returnvalue (Utilities|Time|GetGameTimeinSeconds))
  (Variables|Default|SetHitEndWallTime _returnvalue)
  (Development|PrintString (Utilities|String|ToString(Float) _returnvalue)))

(event OnComponentBeginOverlap(Box)
  (params (OtherActor :type Actor%20Object%20Reference) (OtherComp :type Primitive%20Component%20Object%20Reference) (OtherBodyIndex :type Integer) (bFromSweep :type Boolean) (SweepResult :type Hit%20Result%20Structure%20%28by%20ref%29))
  (Utilities|Casting|CastToBPPhysicsTester OtherActor
    (:CastFailed
      (Variables|Default|SetHitBottomWallTime (Utilities|Time|GetGameTimeinSeconds))
      (CallFunction|FirePLunger))))

(event Custom|ResetPlunger
  (bind _newvar_1 (Variables|Default|GetNewVar_1))
  (Utilities|FlowControl|Sequence
    (:then_0
      (bind _newtrack_0 (Timeline|Timeline_0 Reverse)
        (:Update
          (Transformation|SetRelativeLocation (Variables|Default|Getplunger) (Math|Vector|Lerp(Vector) _newvar_1 (Math|Vector|MakeVector (+ (.X (Math|Vector|BreakVector _newvar_1)) (Variables|Default|GetPlungerMoveDist)) 0.0 -9e+01) _newtrack_0) false false))
        (:Finished
          (CallFunction|ResetPlunger))))
    (:then_1
      (Utilities|FlowControl|Gate false) ; enters at Open
    )))

(event Custom|FirePLunger
  (bind _newvar_1 (Variables|Default|GetNewVar_1))
  (Utilities|FlowControl|Sequence
    (:then_0
      (Utilities|FlowControl|Gate false :!label _label
        (:Exit
          (bind _newtrack_0 (Timeline|Timeline_0 Play)
            (:Update
              (Transformation|SetRelativeLocation (Variables|Default|Getplunger) (Math|Vector|Lerp(Vector) _newvar_1 (Math|Vector|MakeVector (+ (.X (Math|Vector|BreakVector _newvar_1)) (Variables|Default|GetPlungerMoveDist)) 0.0 -9e+01) _newtrack_0) false false))
            (:Finished
              (CallFunction|ResetPlunger))))))
    (:then_1
      (goto _label Close))))

(event EventBeginPlay
  (Game|SpawnActorfromClass "/Game/Blueprints/BasePinball.BasePinball_C" (Transformation|GetWorldTransform (Variables|Default|GetBallSpawn)) "AlwaysSpawn" 0 0)
  (bind _output_get (Variables|Default|SetSpawnedBall 0))
  (Class|PrimitiveComponent|SetLinearDamping (Variables|/Script/Pinball.PinballBall|GetBall _output_get) (Variables|PhysTable|GetBallLinearDamping))
  (Class|PrimitiveComponent|SetAngularDamping (Variables|/Script/Pinball.PinballBall|GetBall _output_get) (Variables|PhysTable|GetBallAngularDamping))
  (Rendering|Material|CreateDynamicMaterialInstance (Variables|/Script/Pinball.PinballBall|GetBall _output_get) 0 (Variables|PhysTable|GetBallMaterial) :!class /Script/Engine.PrimitiveComponent))

(event Collision|EventActorBeginOverlap
  (params (OtherActor :type Actor%20Object%20Reference)))

(event EventTick
  (params (DeltaSeconds :type Float%20%28single-precision%29)))

(fn ConstructionScript
  (Transformation|SetRelativeRotation (Variables|Default|Getroot) (Math|Rotator|MakeRotator 0.0 (Variables|PhysTable|GetTableAngle) 0.0) false false)
  (Components|Timeline|SetPlayRate (Variables|Default|GetTimeline_0) (/ (Variables|PhysTable|GetPlungerSpeed) 1.0))
  (Variables|Default|SetNewVar_1 (Variables|/Script/Engine.SceneComponent|GetRelativeLocation (Variables|Default|Getplunger))))