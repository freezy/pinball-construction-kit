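; Pinball spinner target: a physics tile hung on a rod between two brackets that scores when a ball spins it.
; When a BasePinball hits the tile, it waits briefly and calls RegisterScore on its ScoreComponent only if the tile's angular speed passes a threshold.
; The construction script fits brackets, rod, constraint and tile to an editable end point and heights, and applies tile width and a custom texture via dynamic material.
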(event OnComponentHit(Tile)
  (params (HitComponent :type Primitive%20Component%20Object%20Reference) (OtherActor :type Actor%20Object%20Reference) (OtherComp :type Primitive%20Component%20Object%20Reference) (NormalImpulse :type Vector :default "0, 0, 0") (Hit :type Hit%20Result%20Structure%20%28by%20ref%29))
  (Utilities|Casting|CastToBasePinball OtherActor)
  (Utilities|FlowControl|Delay 0.2)
  (bind _returnvalue (Physics|GetPhysicsAngularVelocityinDegrees (Variables|Default|GetTile) "None"))
  (if (>= (Math|Vector|VectorLength _returnvalue) 45.0)
    (Default|RegisterScore (Variables|Default|GetScoreComponent))))

(event EventBeginPlay)

(event EventActorBeginOverlap
  (params (OtherActor :type Actor%20Object%20Reference)))

(event EventTick
  (params (DeltaSeconds :type Float%20%28single-precision%29)))

(fn ConstructionScript
  (bind _returnvalue (Math|Vector|MakeVector 0.0 0.0 0.0))
  (bind _bracketendpoint (Variables|Default|GetBracketEndPoint))
  (bind _bracketendpoint_2 (Variables|Default|GetBracketEndPoint))
  (bind _spinnerclearanceheight (Variables|Default|GetSpinnerClearanceHeight))
  (bind _bracketheight (Variables|Default|GetBracketHeight))
  (bind _tile (Variables|Default|GetTile))
  (bind _returnvalue_2 (- _spinnerclearanceheight _bracketheight))
  (bind (_x _y) (Math|Vector|BreakVector _bracketendpoint_2))
  (bind _returnvalue_3 (Math|Vector|MakeVector _x _y 0.0))
  (bind _returnvalue_4 (- _returnvalue _returnvalue_3))
  (bind _returnvalue_5 (Math|Vector|VectorLength _returnvalue_4))
  (Transformation|SetRelativeLocation (Variables|Default|GetRotateroot) (Math|Vector|MakeVector 0.0 0.0 (Variables|Default|GetBracketHeight)) false false)
  (Transformation|SetRelativeLocation (Variables|Default|Get2ndBracket) (Math|Vector|MakeVector (.x _bracketendpoint) (.y _bracketendpoint) (Variables|Default|GetBracketHeight)) false false)
  (Transformation|SetRelativeLocation (Variables|Default|GetCylinderRod) (Math|Vector|MakeVector 2e+01 0.0 _returnvalue_2) false false)
  (Transformation|SetRelativeScale3D (Variables|Default|GetSM_BracketTop) (Math|Vector|MakeVector (/ (- _returnvalue_5 4e+01) 1e+02) 1.0 1.0))
  (Transformation|SetRelativeLocation _tile (Math|Vector|MakeVector (/ _returnvalue_5 2.0) 0.0 _returnvalue_2) false false)
  (Transformation|SetRelativeScale3D _tile (Math|Vector|MakeVector (Variables|Default|GetTileWidthMultiplier) 1.0 1.0))
  (Transformation|SetRelativeRotation (Variables|Default|GetRotateroot) (Math|Rotator|FindLookatRotation _returnvalue _returnvalue_3) false false)
  (Transformation|SetRelativeRotation (Variables|Default|Get2ndBracket) (Math|Rotator|FindLookatRotation _returnvalue_3 _returnvalue) false false)
  (Transformation|SetRelativeScale3D (Variables|Default|GetSM_LBracket) (Math|Vector|MakeVector 1.0 1.0 (/ (+ (Variables|Default|GetSpinnerClearanceHeight) -1e+01) 1e+02)))
  (bind _returnvalue_6 (Rendering|Material|CreateDynamicMaterialInstance (Variables|Default|GetTile) 0 0 "None" :!class /Script/Engine.PrimitiveComponent))
  (Rendering|Material|SetTextureParameterValue _returnvalue_6 "CustomSpinnerTexture" (Variables|Default|GetSpinnerTexture)))