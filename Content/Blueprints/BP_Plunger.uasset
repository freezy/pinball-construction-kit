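; Pinball plunger actor that loads balls and launches them into play.
; LoadBall spawns a GamePinball at the spawn point, stores the auto-shot flag and plays a reset sound.
; When the ball overlaps the box, it either auto-fires after a short delay or activates the plunger on the PinballPlayerController.
; ShootBall applies a Y impulse with a sound, using fixed full power for multiball auto-shots and the supplied power for player shots.
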(event OnComponentBeginOverlap(Box)
  (params (OtherActor :type Actor%20Object%20Reference) (OtherComp :type Primitive%20Component%20Object%20Reference) (OtherBodyIndex :type Integer) (bFromSweep :type Boolean) (SweepResult :type Hit%20Result%20Structure%20%28by%20ref%29))
  (bind _asgame_pinball (Utilities|Casting|CastToGamePinball OtherActor))
  (Variables|Default|SetLoadedBall _asgame_pinball)
  (if (Variables|Default|GetAutoShot)
    (Utilities|FlowControl|Delay 0.5)
    (CallFunction|ShootBall 0.0)
    (else
      (bind _aspinball_player_controller (Utilities|Casting|CastToPinballPlayerController (Game|GetPlayerController 0)))
      (Variables|/Game/Blueprints/PinballPlayerController.PinballPlayerController_C|SetPlungerActive _aspinball_player_controller true))))

(event Custom|ShootBall
  (params (ShootPower :type Float%20%28single-precision%29))
  (Physics|AddImpulse (Variables|/Script/Pinball.PinballBall|GetBall (Variables|Default|GetLoadedBall)) (Math|Vector|MakeVector 0.0 (Math|Float|SelectFloat -3e+04 ShootPower (Variables|Default|GetAutoShot)) 0.0) "None" false)
  (Audio|PlaySoundatLocation "/Game/Assets/Audio/Arcade_Enemy_Death_01_m1.Arcade_Enemy_Death_01_m1" (Transformation|GetWorldLocation (Variables|Default|GetSM_Plunger))))

(event Custom|LoadBall
  (params (AutoShot :type Boolean))
  (bind _ballspawnpoint (Variables|Default|GetBallSpawnPoint))
  (bind _returnvalue (Transformation|GetWorldLocation _ballspawnpoint))
  (Variables|Default|SetAutoShot AutoShot)
  (Game|SpawnActorfromClass "/Game/Blueprints/GamePinball.GamePinball_C" (Math|Conversions|ToTransform(Vector) _returnvalue) "AlwaysSpawn" 0 0)
  (Audio|PlaySoundatLocation "/Game/Sounds/Pinball_Reset02.Pinball_Reset02" _returnvalue))

(event EventBeginPlay)

(event EventActorBeginOverlap
  (params (OtherActor :type Actor%20Object%20Reference)))

(event EventTick
  (params (DeltaSeconds :type Float%20%28single-precision%29)))

(fn ConstructionScript)