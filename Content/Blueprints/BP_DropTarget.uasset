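; Pinball drop target that drops when struck by a ball, registers score and can be reset.
; The first ball hit plays a sound, lowers the target, disables its collision, activates the linked object and reports its index.
; Reset raises it, restores collision, deactivates that object and rearms the hit gate.
; A dynamic material built from TargetData sets colors and textures, both at construction and BeginPlay.
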(event OnComponentHit(Target)
  (params (OtherActor :type Actor%20Object%20Reference) (OtherComp :type Primitive%20Component%20Object%20Reference) (NormalImpulse :type Vector :default "0, 0, 0") (Hit :type Hit%20Result%20Structure%20%28by%20ref%29))
  (bind _target (Variables|Default|GetTarget))
  (Utilities|Casting|CastToBasePinball OtherActor)
  (if (not (Variables|Default|GetTargetDown))
    (Utilities|FlowControl|DoOnce false
      (:Completed
        (Audio|SpawnSoundAttached "/Game/Sounds/Arcade_Enemy_Death_03_m1.Arcade_Enemy_Death_03_m1" _target)
        (Components|MoveComponentTo _target "0, 0,-120.000000" "0, 0, 0" false false 0.1)
        (Collision|SetCollisionEnabled (Variables|Default|GetTarget) "NoCollision")
        (Variables|Default|SetTargetDown true)
        (Class|PinballInterface|Activate(Message) (.objecttoactivate (Variables|Default|GetTargetData)))
        (Default|CallTargetHit (Variables|Default|GetTargetIndex))
        (Default|RegisterScore (Variables|Default|GetScoreComponent))))))

(event Custom|Reset
  (bind _targetdata (Variables|Default|GetTargetData))
  (bind _target (Variables|Default|GetTarget))
  (Components|MoveComponentTo (Variables|Default|GetTarget) "0, 0,-10.000000" "0, 0, 0" false false 0.1)
  (Collision|SetCollisionEnabled (Variables|Default|GetTarget) "QueryAndPhysics")
  (Variables|Default|SetTargetDown false)
  (Class|PinballInterface|Deactivate(Message) (.objecttoactivate _targetdata))
  (Utilities|FlowControl|DoOnce false) ; enters at Reset
)

(event EventBeginPlay
  (CallFunction|SetTargetStyle))

(event Collision|EventActorBeginOverlap
  (params (OtherActor :type Actor%20Object%20Reference)))

(event EventTick
  (params (DeltaSeconds :type Float%20%28single-precision%29)))

(fn ConstructionScript
  (CallFunction|SetTargetStyle))

(fn SetTargetStyle
  (params (Texture :type Texture%202D%20Object%20Reference))
  (bind _targetdata (Variables|Default|GetTargetData))
  (bind _returnvalue (Rendering|Material|CreateDynamicMaterialInstance (Variables|Default|GetTarget) 0 "/Game/Materials/M_DropTargetBase.M_DropTargetBase" :!class /Script/Engine.PrimitiveComponent))
  (Utilities|FlowControl|Sequence
    (:then_0
      (Rendering|Material|SetVectorParameterValue _returnvalue "BaseColor" (.basecolor _targetdata) :!class /Script/Engine.MaterialInstanceDynamic))
    (:then_1
      (Rendering|Material|SetVectorParameterValue _returnvalue "TargetColor" (.targetcolor _targetdata) :!class /Script/Engine.MaterialInstanceDynamic))
    (:then_2
      (Rendering|Material|SetVectorParameterValue _returnvalue "LetterColor" (.lettercolor _targetdata) :!class /Script/Engine.MaterialInstanceDynamic))
    (:then_3
      (Rendering|Material|SetTextureParameterValue _returnvalue "TargetLetterTexture" (Utilities|Array|Get(acopy) (Variables|Default|GetTargetTextures) (Math|Conversions|ToInteger(Byte) (.targetstyle _targetdata)))))
    (:then_4
      (Rendering|Material|SetTextureParameterValue _returnvalue "CustomTargetTexture" (.droptargettexture _targetdata)))))