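; BP_Indicator_Special is a child indicator Blueprint that takes its icon and light color from a selected special mode.
; The construction script indexes SpecialModeStruct by the SpecialType enum to set IconTexture and LightColor before running the parent construction script.
; Activate and Deactivate only forward to the parent, which handles the indicator's behavior.
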(event EventBeginPlay
  (|CallParentFunction))

(event EventActorBeginOverlap
  (params (OtherActor :type Actor%20Object%20Reference)))

(event EventTick
  (params (DeltaSeconds :type Float%20%28single-precision%29)))

(event EventActivate
  (|CallParentFunction))

(event EventDeactivate
  (|CallParentFunction))

(fn ConstructionScript
  (bind _specialtype (Variables|IndicatorSpecial|GetSpecialType))
  (bind _specialmodestruct (Variables|Default|GetSpecialModeStruct))
  (bind _returnvalue (Math|Conversions|ToInteger(Byte) _specialtype))
  (bind _item (Utilities|Array|Get(acopy) _specialmodestruct _returnvalue))
  (Variables|Default|SetIconTexture (.modetexture _item))
  (Variables|Default|SetLightColor (.modecolor _item))
  (|CallParentFunction))