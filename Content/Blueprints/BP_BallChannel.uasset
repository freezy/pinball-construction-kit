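; BP_BallChannel is an actor that builds a configurable row of ball channel static meshes, with no active runtime logic.
; The Construction Script adds Count mesh components along local X, stepping each by 100 units plus Spacing.
; Each mesh gets BaseMaterial on its first slot and a dynamic material instance on its second, tinted by RubberColor through the BaseColor parameter.
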(event EventBeginPlay)

(event EventActorBeginOverlap
  (params (OtherActor :type Actor%20Object%20Reference)))

(event EventTick
  (params (DeltaSeconds :type Float%20%28single-precision%29)))

(fn ConstructionScript
  (for _index (range 0 (- (Variables|Default|GetCount) 1))
    (bind _returnvalue (AddComponent|AddStaticMeshComponent false (Math|Transform|MakeTransform (Math|Vector|MakeVector (* _index (+ (Variables|Default|GetSpacing) 1e+02)) 0.0 0.0) "0, 0, 0" "1,1,1")))
    (Rendering|Material|SetMaterial _returnvalue 0 (Variables|Default|GetBaseMaterial))
    (bind _returnvalue_2 (Rendering|Material|CreateDynamicMaterialInstance _returnvalue 1 0 :!class /Script/Engine.PrimitiveComponent))
    (Rendering|Material|SetVectorParameterValue _returnvalue_2 "BaseColor" (Variables|Default|GetRubberColor) :!class /Script/Engine.MaterialInstanceDynamic)))